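; Glock weapon for BP_FPSPawn, handling firing, timed reload, aim down sights and saving its stats to the pawn's secondary slot on unequip.
; Fire spends ammo, traces from the camera with random spread, then spawns an impact decal, an occasional tracer and a muzzle flash, without applying damage.
; A second muzzle-to-impact trace runs but its result is unused.
; Timelines blend camera FOV and arms position for aiming.
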(event EventUnequip
  (Variables|/Game/FPS_Tut/Blueprints/BP_FPSPawn.BP_FPSPawn_C|SetSecondaryWeapon (.AsBP%20FPSPawn (Utilities|Casting|CastToBP_FPSPawn (Game|GetPlayerCharacter 0))) (Utilities|Struct|MakeWeaponData "NewEnumerator2" "Weapon_Glock_C" (Variables|Default|GetAmmoCount) (Variables|Default|GetMaxAmmo) (Variables|Default|GetReloadTime) (Variables|Default|GetBulletSpread))))

(event EventReload
  (bind _returnvalue (Game|GetPlayerCharacter 0))
  (bind _asbp_fpspawn (Utilities|Casting|CastToBP_FPSPawn _returnvalue))
  (if (< (Variables|Default|GetAmmoCount) (Variables|Default|GetMaxAmmo))
    (Utilities|FlowControl|DoOnce false :!label _label
      (:Completed
        (Variables|/Game/FPS_Tut/Blueprints/BP_FPSPawn.BP_FPSPawn_C|SetIsReloading _asbp_fpspawn true)
        (Animation|Montage|MontagePlay (Components|SkeletalMesh|GetAnimInstance (Variables|/Game/FPS_Tut/Blueprints/BP_FPSPawn.BP_FPSPawn_C|GetFirstPersonMesh _asbp_fpspawn)) "/Game/FPS_Tut/Animations/Arms_Glock_Reload_anim_Montage.Arms_Glock_Reload_anim_Montage" 1.0 "MontageLength" 0.0 true)
        (Components|Animation|PlayAnimation (Variables|Default|GetPrimaryWeapon) "/Game/FPS_Tut/Animations/Arms_Glock_Reload_anim_Montage.Arms_Glock_Reload_anim_Montage" false)
        (Utilities|FlowControl|Delay (Variables|Default|GetReloadTime))
        (Variables|Default|SetAmmoCount (Variables|Default|GetMaxAmmo))
        (Variables|/Game/FPS_Tut/Blueprints/BP_FPSPawn.BP_FPSPawn_C|SetIsReloading _asbp_fpspawn false)
        (goto _label Reset)))))

(event EventFire
  (bind _returnvalue (Game|GetPlayerCharacter 0))
  (bind _asbp_fpspawn (Utilities|Casting|CastToBP_FPSPawn _returnvalue))
  (bind _firstpersonmesh (Variables|/Game/FPS_Tut/Blueprints/BP_FPSPawn.BP_FPSPawn_C|GetFirstPersonMesh _asbp_fpspawn))
  ;[1 1 1] Ammo Check
  (if (> (Variables|Default|GetAmmoCount) 0)
    (CallFunction|AmmoCheck)
    (bind (_muzzleloc _impact_point) (CallFunction|LineTrace))
    (CallFunction|SpawnDecalTracer _muzzleloc _impact_point _impact_point)
    (if (Variables|/Game/FPS_Tut/Blueprints/BP_FPSPawn.BP_FPSPawn_C|GetAimDownSight _asbp_fpspawn)
      (Animation|Montage|PlayMontage _firstpersonmesh "/Game/FPS_Tut/Animations/Arms_Glock_ADS_Fire_anim_Montage.Arms_Glock_ADS_Fire_anim_Montage"
        (:then
          _))
      (else
        (Animation|Montage|PlayMontage _firstpersonmesh "/Game/FPS_Tut/Animations/Arms_Glock_Fire_anim_Montage.Arms_Glock_Fire_anim_Montage"
          (:then
            _))))
    (Utilities|MuzzleFlash)
    (else
      (Audio|PlaySoundatLocation "/Game/FPS_Tut/SoundFX/DryFire.DryFire" (Transformation|GetWorldLocation (Variables|/Game/FPS_Tut/Blueprints/BP_FPSPawn.BP_FPSPawn_C|GetFirstPersonCamera (.AsBP%20FPSPawn (Utilities|Casting|CastToBP_FPSPawn (Game|GetPlayerCharacter 0))))) "0, 0, 0" 1.0 1.0 0.0 0 0 0 0))))

(event EventAimDownSight
  (params (Toggle :type Boolean))
  (bind _returnvalue (Game|GetPlayerCharacter 0))
  (bind _asbp_fpspawn (Utilities|Casting|CastToBP_FPSPawn _returnvalue))
  (bind _firstpersoncamera (Variables|/Game/FPS_Tut/Blueprints/BP_FPSPawn.BP_FPSPawn_C|GetFirstPersonCamera _asbp_fpspawn))
  (bind _firstpersonmesh (Variables|/Game/FPS_Tut/Blueprints/BP_FPSPawn.BP_FPSPawn_C|GetFirstPersonMesh _asbp_fpspawn))
  ;[1 1 1] Aim Down Sight
  (if Toggle
    (bind _float (Timeline|Timeline_0 PlayFromStart)
      (:Update
        (Camera|SetFieldOfView _firstpersoncamera (Math|Float|Lerp 9e+01 55.0 _float))
        (Transformation|SetRelativeTransform _firstpersonmesh (Math|Transform|MakeTransform (Math|Vector|Lerp(Vector) "0.000000,0.000000,-20.000000" "0.000000,0.050000,-15.600000" _float) "-0.100000,-1.270000,0.000000" "1.000000,1.000000,1.000000") false false)))
    (else
      (bind _float_2 (Timeline|Timeline_1 PlayFromStart)
        (:Update
          (Camera|SetFieldOfView _firstpersoncamera (Math|Float|Lerp 55.0 9e+01 _float_2))
          (Transformation|SetRelativeTransform _firstpersonmesh (Math|Transform|MakeTransform (Math|Vector|Lerp(Vector) "0.000000,0.050000,-15.600000" "0.000000,0.000000,-20.000000" _float_2) "0, 0, 0" "1.000000,1.000000,1.000000") false false))))))

(fn ConstructionScript
  (|CallParentFunction)
  (Variables|Default|SetMaxAmmo 11)
  (Variables|Default|SetAmmoCount 11)
  (Variables|Default|SetReloadTime 1.5)
  (Variables|Default|SetBulletSpread 175.0)
  (Variables|Default|SetName "NewEnumerator2")
  (Variables|Default|SetVariableFire false))

(fn AmmoCheck
  (bind _returnvalue (Math|Random|RandomFloatinRange 0.7 1.2))
  ;[1 1 1] Deplete Ammo
  (Math|Integer|DecrementInt (Variables|Default|GetAmmoCount)
    (:%20%20
      (Audio|PlaySoundatLocation "/Game/FPS_Tut/SoundFX/vandalTap.vandalTap" (Transformation|GetActorLocation) "0, 0, 0" (+ _returnvalue 2.5) _returnvalue 0.0 0 0 0 0)
      (Components|Animation|PlayAnimation (Variables|Default|GetPrimaryWeapon) "/Game/FPS_Tut/Animations/Glock_Fire_anim.Glock_Fire_anim" false))))

(fn LineTrace
  (bind _returnvalue (Game|GetPlayerCharacter 0))
  (bind _bulletspread (Variables|Default|GetBulletSpread))
  (bind _muzzle (Variables|Default|GetMuzzle))
  (bind _returnvalue_2 (Transformation|GetWorldLocation _muzzle))
  (bind _asbp_fpspawn (Utilities|Casting|CastToBP_FPSPawn _returnvalue))
  (bind _returnvalue_3 (* _bulletspread -1.0))
  (bind _firstpersoncamera (Variables|/Game/FPS_Tut/Blueprints/BP_FPSPawn.BP_FPSPawn_C|GetFirstPersonCamera _asbp_fpspawn))
  (bind _returnvalue_4 (Transformation|GetWorldLocation _firstpersoncamera))
  ;[1 1 1] Basic Line Tracing
  ;[1 1 1] Visual Line Trace
  (bind _outhit (Collision|LineTraceByChannel _returnvalue_4 (+ (+ _returnvalue_4 (* (Math|Vector|GetForwardVector _firstpersoncamera) 2e+04)) (Math|Vector|MakeVector (Math|Random|RandomFloatinRange _returnvalue_3 _bulletspread) (Math|Random|RandomFloatinRange _returnvalue_3 _bulletspread) (Math|Random|RandomFloatinRange _returnvalue_3 _bulletspread))) "TraceTypeQuery1" false 0 "None")) ; Line Trac Fire Fom Camera
  (Collision|LineTraceByChannel _returnvalue_2 (.ImpactPoint (Collision|BreakHitResult _outhit)) "TraceTypeQuery1" false 0 "None" true "(R=0.000000,G=0.000000,B=1.000000,A=1.000000)") ; Line Trace Fire Fom Weapon
  (return _returnvalue_2 (.ImpactPoint (Collision|BreakHitResult _outhit))))

(fn SpawnDecalTracer
  (params (Location :type Vector) (SpawnTransformLocation :type Vector) (ImpactPoint :type Vector))
  (Game|SpawnActorfromClass "/Game/FPS_Tut/Blueprints/BP_BulletDecal.BP_BulletDecal_C" (Math|Transform|MakeTransform SpawnTransformLocation (Math|Conversions|RotationFromXVector ImpactPoint) "0.025000,0.025000,0.025000") "Undefined" 0 0)
  (if (> (Math|Random|RandomIntegerinRange 1 10) 5)
    (Game|SpawnActorfromClass "/Game/FPS_Tut/Blueprints/BP_TracerRound.BP_TracerRound_C" (Math|Transform|MakeTransform Location (Transformation|GetWorldRotation (Variables|/Game/FPS_Tut/Blueprints/BP_FPSPawn.BP_FPSPawn_C|GetFirstPersonCamera (.AsBP%20FPSPawn (Utilities|Casting|CastToBP_FPSPawn (Game|GetPlayerCharacter 0))))) "0.050000,0.050000,0.050000") "Undefined" 0 0))
  (return))