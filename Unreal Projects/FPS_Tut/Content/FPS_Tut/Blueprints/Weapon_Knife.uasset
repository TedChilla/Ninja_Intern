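; Melee knife weapon for the FPS player pawn, a child Blueprint that overrides its parent's setup to act as a non-automatic weapon.
; Fire, gated by a short retriggerable cooldown, plays one of three random first-person attack montages and runs a short, spread-jittered camera trace.
; The trace result feeds a knife decal spawn, oriented by camera yaw on upward-facing floors and by impact normal elsewhere, with no damage applied.
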(event EventFire
  (bind _returnvalue (Game|GetPlayerCharacter 0))
  (bind _asbp_fpspawn (Utilities|Casting|CastToBP_FPSPawn _returnvalue))
  (bind _firstpersonmesh (Variables|/Game/FPS_Tut/Blueprints/BP_FPSPawn.BP_FPSPawn_C|GetFirstPersonMesh _asbp_fpspawn))
  (if (not (Variables|Default|GetCooldown))
    (Variables|Default|SetCooldown true)
    (Utilities|FlowControl|Sequence
      (:then_0
        (switch int (Math|Random|RandomIntegerinRange 0 2)
          (:0
            (Animation|Montage|PlayMontage _firstpersonmesh "/Game/FPS_Tut/Animations/Arms_Knife_Attack_01_anim_Montage.Arms_Knife_Attack_01_anim_Montage"))
          (:1
            (Animation|Montage|PlayMontage _firstpersonmesh "/Game/FPS_Tut/Animations/Arms_Knife_Attack_02_anim_Montage.Arms_Knife_Attack_02_anim_Montage"))
          (:2
            (Animation|Montage|PlayMontage _firstpersonmesh "/Game/FPS_Tut/Animations/Arms_Knife_Attack_03_anim_Montage.Arms_Knife_Attack_03_anim_Montage"))))
      (:then_1
        (bind (_impact_normal _impact_point) (CallFunction|LineTrace))
        (CallFunction|SpawnDecalTracer _impact_normal _impact_point))
      (:then_2
        (Utilities|FlowControl|RetriggerableDelay 0.5)
        (Variables|Default|SetCooldown false)))))

(fn ConstructionScript
  (|CallParentFunction)
  (Variables|Default|SetName "NewEnumerator0")
  (Variables|Default|SetVariableFire false))

(fn LineTrace
  (bind _returnvalue (Game|GetPlayerCharacter 0))
  (bind _bulletspread (Variables|Default|GetBulletSpread))
  (bind _asbp_fpspawn (Utilities|Casting|CastToBP_FPSPawn _returnvalue))
  (bind _returnvalue_2 (* _bulletspread -1.0))
  (bind _firstpersoncamera (Variables|/Game/FPS_Tut/Blueprints/BP_FPSPawn.BP_FPSPawn_C|GetFirstPersonCamera _asbp_fpspawn))
  (bind _returnvalue_3 (Transformation|GetWorldLocation _firstpersoncamera))
  ;[1 1 1] Basic Line Tracing
  ;[1 1 1] Visual Line Trace
  (bind (_outhit _returnvalue_4) (Collision|LineTraceByChannel _returnvalue_3 (+ (+ _returnvalue_3 (* (Math|Vector|GetForwardVector _firstpersoncamera) 175.0)) (Math|Vector|MakeVector (Math|Random|RandomFloatinRange _returnvalue_2 _bulletspread) (Math|Random|RandomFloatinRange _returnvalue_2 _bulletspread) (Math|Random|RandomFloatinRange _returnvalue_2 _bulletspread))) "TraceTypeQuery1" false 0 "None")) ; Line Trac Fire Fom Camera
  (if _returnvalue_4
    (return (.ImpactNormal (Collision|BreakHitResult _outhit)) (.ImpactPoint (Collision|BreakHitResult _outhit)))))

(fn SpawnDecalTracer
  (params (ImpactNormal :type Vector) (ImpactPoint :type Vector))
  (bind _returnvalue (Math|Conversions|RotationFromXVector ImpactNormal))
  (bind _returnvalue_2 (Game|GetPlayerCharacter 0))
  (bind _asbp_fpspawn (Utilities|Casting|CastToBP_FPSPawn _returnvalue_2))
  (bind _firstpersoncamera (Variables|/Game/FPS_Tut/Blueprints/BP_FPSPawn.BP_FPSPawn_C|GetFirstPersonCamera _asbp_fpspawn))
  (if (Utilities|Operators|EqualEqual ImpactNormal "0,0,1.000000" 0.0)
    (Game|SpawnActorfromClass "/Game/FPS_Tut/Blueprints/BP_KnifeDecal.BP_KnifeDecal_C" (Math|Transform|MakeTransform ImpactPoint (Math|Rotator|MakeRotator -9e+01 9e+01 (.yaw (Math|Conversions|RotationFromXVector (Math|Vector|GetForwardVector _firstpersoncamera)))) "0.100000,0.080000,0.080000") "Undefined" 0 0)
    (else
      (Game|SpawnActorfromClass "/Game/FPS_Tut/Blueprints/BP_KnifeDecal.BP_KnifeDecal_C" (Math|Transform|MakeTransform ImpactPoint (Math|Rotator|MakeRotator (+ (.roll (Transformation|GetWorldRotation _firstpersoncamera)) 9e+01) (.pitch _returnvalue) (+ (.yaw _returnvalue) 1.8e+02)) "0.100000,0.080000,0.080000") "Undefined" 0 0)))
  (return))