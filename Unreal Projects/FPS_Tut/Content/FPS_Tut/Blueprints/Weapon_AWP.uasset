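; Weapon_AWP is a scoped sniper rifle for the first-person pawn, with a small magazine, fire, reload and aim-down-sight.
; Aiming uses timelines to lerp camera FOV and arm position, then hides arms and gun behind an HUD_Scope widget.
; Firing unscopes, line-traces from the camera with random spread, spawns decals and occasional tracers, and re-scopes on montage blend-out if still aiming.
; Reload is DoOnce-guarded and refills ammo after a delay.
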(event EventReload
  (bind _returnvalue (Game|GetPlayerCharacter 0))
  (bind _asbp_fpspawn (Utilities|Casting|CastToBP_FPSPawn _returnvalue))
  (if (< (Variables|Default|GetAmmoCount) (Variables|Default|GetMaxAmmo))
    (Utilities|FlowControl|DoOnce false :!label _label
      (:Completed
        (Variables|/Game/FPS_Tut/Blueprints/BP_FPSPawn.BP_FPSPawn_C|SetIsReloading _asbp_fpspawn true)
        (Animation|Montage|MontagePlay (Components|SkeletalMesh|GetAnimInstance (Variables|/Game/FPS_Tut/Blueprints/BP_FPSPawn.BP_FPSPawn_C|GetFirstPersonMesh _asbp_fpspawn)) "/Game/FPS_Tut/Animations/Arms_AWP_Reload_anim_Montage.Arms_AWP_Reload_anim_Montage" 1.0 "MontageLength" 0.0 true)
        (Components|Animation|PlayAnimation (Variables|Default|GetPrimaryWeapon) "/Game/FPS_Tut/Animations/AWP_Reload_anim_Montage.AWP_Reload_anim_Montage" false)
        (Utilities|FlowControl|Delay (Variables|Default|GetReloadTime))
        (Variables|Default|SetAmmoCount (Variables|Default|GetMaxAmmo))
        (Variables|/Game/FPS_Tut/Blueprints/BP_FPSPawn.BP_FPSPawn_C|SetIsReloading _asbp_fpspawn false)
        (goto _label Reset)))))

(event EventBeginPlay
  (bind _returnvalue (UserInterface|CreateWidget "/Game/FPS_Tut/Blueprints/HUD_Scope.HUD_Scope_C"))
  (Variables|Default|SetHUD%20Scope _returnvalue))

(event EventFire
  (bind _returnvalue (Game|GetPlayerCharacter 0))
  (bind _returnvalue_2 (Game|GetPlayerCharacter 0))
  (bind _hud_scope (Variables|Default|GetHUD%20Scope))
  (bind _asbp_fpspawn (Utilities|Casting|CastToBP_FPSPawn _returnvalue))
  (bind _asbp_fpspawn_2 (Utilities|Casting|CastToBP_FPSPawn _returnvalue_2))
  (bind _firstpersonmesh (Variables|/Game/FPS_Tut/Blueprints/BP_FPSPawn.BP_FPSPawn_C|GetFirstPersonMesh _asbp_fpspawn_2))
  (bind _firstpersoncamera (Variables|/Game/FPS_Tut/Blueprints/BP_FPSPawn.BP_FPSPawn_C|GetFirstPersonCamera _asbp_fpspawn))
  (if (Variables|Default|GetCanFire)
    (Variables|Default|SetCanFire false)
    (if (> (Variables|Default|GetAmmoCount) 0)
      (Camera|SetFieldOfView (Variables|/Game/FPS_Tut/Blueprints/BP_FPSPawn.BP_FPSPawn_C|GetFirstPersonCamera _asbp_fpspawn_2) 9e+01)
      (Transformation|SetRelativeTransform _firstpersonmesh (Math|Transform|MakeTransform "6.400000,5.500000,-23.600000" "0,6.400000, 0" "1.000000,1.000000,1.000000") false false)
      (Rendering|SetVisibility _firstpersonmesh true false)
      (Widget|SetVisibility (Variables|Default|GetHUD%20Scope) "Hidden")
      (CallFunction|AmmoCheck)
      (bind (_muzzleloc _impact_point) (CallFunction|LineTrace))
      (CallFunction|SpawnDecalTracer _muzzleloc _impact_point _impact_point)
      (Animation|Montage|PlayMontage (Variables|/Game/FPS_Tut/Blueprints/BP_FPSPawn.BP_FPSPawn_C|GetFirstPersonMesh _asbp_fpspawn) "/Game/FPS_Tut/Animations/Arms_AWP_Fire_anim_Montage.Arms_AWP_Fire_anim_Montage"
        (:then
          (Utilities|MuzzleFlash))
        (:OnBlendOut
          (Variables|Default|SetCanFire true)
          (if (Variables|/Game/FPS_Tut/Blueprints/BP_FPSPawn.BP_FPSPawn_C|GetAimDownSight _asbp_fpspawn)
            (Rendering|SetVisibility (Variables|/Game/FPS_Tut/Blueprints/BP_FPSPawn.BP_FPSPawn_C|GetFirstPersonMesh _asbp_fpspawn) false false)
            (Widget|SetVisibility _hud_scope "Visible")
            (Camera|SetFieldOfView _firstpersoncamera (Variables|Default|GetAimDownSight_FOV))
            (else
              (Rendering|SetVisibility (Variables|/Game/FPS_Tut/Blueprints/BP_FPSPawn.BP_FPSPawn_C|GetGun _asbp_fpspawn) true false)
              (Widget|SetVisibility _hud_scope "Hidden")
              (Camera|SetFieldOfView _firstpersoncamera 9e+01)))))
      (else
        (Audio|PlaySound2D "/Game/FPS_Tut/SoundFX/DryFire.DryFire" 1.0 1.0 0.0 0 0)))))

(event EventAimDownSight
  (params (Toggle :type Boolean))
  (bind _returnvalue (Game|GetPlayerCharacter 0))
  (bind _asbp_fpspawn (Utilities|Casting|CastToBP_FPSPawn _returnvalue))
  (bind _firstpersoncamera (Variables|/Game/FPS_Tut/Blueprints/BP_FPSPawn.BP_FPSPawn_C|GetFirstPersonCamera _asbp_fpspawn))
  (bind _firstpersonmesh (Variables|/Game/FPS_Tut/Blueprints/BP_FPSPawn.BP_FPSPawn_C|GetFirstPersonMesh _asbp_fpspawn))
  ;[1 1 1] Aim Down Sight
  (if Toggle
    (bind _returnvalue_2 (UserInterface|CreateWidget "/Game/FPS_Tut/Blueprints/HUD_Scope.HUD_Scope_C"))
    (bind _output_get (Variables|Default|SetHUD%20Scope _returnvalue_2))
    (UserInterface|Viewport|AddtoViewport _output_get 0)
    (bind _float (Timeline|Timeline_0 PlayFromStart)
      (:Update
        (Camera|SetFieldOfView _firstpersoncamera (Math|Float|Lerp 9e+01 (Variables|Default|GetAimDownSight_FOV) _float))
        (Transformation|SetRelativeTransform _firstpersonmesh (Math|Transform|MakeTransform (Math|Vector|Lerp(Vector) "0.000000,0.000000,-20.000000" "0.000000,0.050000,-15.600000" _float) "0, 0, 0" "1.000000,1.000000,1.000000") false false))
      (:Finished
        (Rendering|SetVisibility _firstpersonmesh false false)))
    (elif (Variables|Default|GetCanFire)
      (Widget|SetVisibility (Variables|Default|GetHUD%20Scope) "Hidden")
      (Rendering|SetVisibility (Variables|/Game/FPS_Tut/Blueprints/BP_FPSPawn.BP_FPSPawn_C|GetFirstPersonMesh _asbp_fpspawn) true false)
      (bind _float_2 (Timeline|Timeline_1 PlayFromStart)
        (:Update
          (Camera|SetFieldOfView _firstpersoncamera (Math|Float|Lerp (Variables|Default|GetAimDownSight_FOV) 9e+01 _float_2))
          (Transformation|SetRelativeTransform _firstpersonmesh (Math|Transform|MakeTransform (Math|Vector|Lerp(Vector) "0.000000,0.050000,-15.600000" "0.000000,0.000000,-20.000000" _float_2) "0, 0, 0" "1.000000,1.000000,1.000000") false false))))))

(event EventUnequip
  (Variables|/Game/FPS_Tut/Blueprints/BP_FPSPawn.BP_FPSPawn_C|SetPrimaryWeapon%20 (.AsBP%20FPSPawn (Utilities|Casting|CastToBP_FPSPawn (Game|GetPlayerCharacter 0))) (Utilities|Struct|MakeWeaponData "NewEnumerator4" "Weapon_AWP_C" (Variables|Default|GetAmmoCount) (Variables|Default|GetMaxAmmo) (Variables|Default|GetReloadTime) (Variables|Default|GetBulletSpread))))

(fn ConstructionScript
  (|CallParentFunction)
  (Variables|Default|SetMaxAmmo 3)
  (Variables|Default|SetAmmoCount 3)
  (Variables|Default|SetReloadTime 2.7)
  (Variables|Default|SetBulletSpread 2e+01)
  (Variables|Default|SetName "NewEnumerator4")
  (Variables|Default|SetVariableFire false))

(fn AmmoCheck
  (bind _returnvalue (Math|Random|RandomFloatinRange 0.7 1.2))
  ;[1 1 1] Deplete Ammo
  (Math|Integer|DecrementInt (Variables|Default|GetAmmoCount)
    (:%20%20
      (Audio|PlaySoundatLocation "/Game/FPS_Tut/SoundFX/vandalTap.vandalTap" (Transformation|GetActorLocation) "0, 0, 0" (+ _returnvalue 2.5) _returnvalue 0.0 0 0 0 0)
      (Components|Animation|PlayAnimation (Variables|Default|GetPrimaryWeapon) "/Game/FPS_Tut/Animations/AWP_Fire_anim.AWP_Fire_anim" false))))

(fn LineTrace
  (bind _returnvalue (Game|GetPlayerCharacter 0))
  (bind _bulletspread (Variables|Default|GetBulletSpread))
  (bind _muzzle (Variables|Default|GetMuzzle))
  (bind _returnvalue_2 (Transformation|GetWorldLocation _muzzle))
  (bind _asbp_fpspawn (Utilities|Casting|CastToBP_FPSPawn _returnvalue))
  (bind _returnvalue_3 (* _bulletspread -1.0))
  (bind _firstpersoncamera (Variables|/Game/FPS_Tut/Blueprints/BP_FPSPawn.BP_FPSPawn_C|GetFirstPersonCamera _asbp_fpspawn))
  (bind _returnvalue_4 (Transformation|GetWorldLocation _firstpersoncamera))
  ;[1 1 1] Basic Line Tracing
  ;[1 1 1] Visual Line Trace
  (bind _outhit (Collision|LineTraceByChannel (+ _returnvalue_4 (Variables|Default|GetAim%20Offset)) (+ (+ _returnvalue_4 (* (Math|Vector|GetForwardVector _firstpersoncamera) 2e+04)) (Math|Vector|MakeVector (Math|Random|RandomFloatinRange _returnvalue_3 _bulletspread) (Math|Random|RandomFloatinRange _returnvalue_3 _bulletspread) (Math|Random|RandomFloatinRange _returnvalue_3 _bulletspread))) "TraceTypeQuery1" false 0 "None")) ; Line Trac Fire Fom Camera
  (Collision|LineTraceByChannel _returnvalue_2 (.ImpactPoint (Collision|BreakHitResult _outhit)) "TraceTypeQuery1" false 0 "None" true "(R=0.000000,G=0.000000,B=1.000000,A=1.000000)") ; Line Trace Fire Fom Weapon
  (return _returnvalue_2 (.ImpactPoint (Collision|BreakHitResult _outhit))))

(fn SpawnDecalTracer
  (params (Location :type Vector) (SpawnTransformLocation :type Vector) (ImpactPoint :type Vector))
  (Game|SpawnActorfromClass "/Game/FPS_Tut/Blueprints/BP_BulletDecal.BP_BulletDecal_C" (Math|Transform|MakeTransform SpawnTransformLocation (Math|Conversions|RotationFromXVector ImpactPoint) "0.025000,0.025000,0.025000") "Undefined" 0 0)
  (if (> (Math|Random|RandomIntegerinRange 1 10) 5)
    (Game|SpawnActorfromClass "/Game/FPS_Tut/Blueprints/BP_TracerRound.BP_TracerRound_C" (Math|Transform|MakeTransform Location (Transformation|GetWorldRotation (Variables|/Game/FPS_Tut/Blueprints/BP_FPSPawn.BP_FPSPawn_C|GetFirstPersonCamera (.AsBP%20FPSPawn (Utilities|Casting|CastToBP_FPSPawn (Game|GetPlayerCharacter 0))))) "0.050000,0.050000,0.050000") "Undefined" 0 0))
  (return))